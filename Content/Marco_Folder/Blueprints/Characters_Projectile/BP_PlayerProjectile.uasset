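; BP_PlayerProjectile is a player projectile that damages actors carrying a health component.
; On BeginPlay it copies its InitialSpeed variable to both the initial and max speed of its ProjectileMovement component.
; When Sphere1 overlaps an actor with AC_Health, it calls TakeDamage with its Damage value and destroys itself.
; Overlaps with actors lacking that component are ignored.
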(event `self.ReceiveBeginPlay`
  (bind _projectilemovement (`self.ProjectileMovement`))
  ;[1 1 1] Set initial speed value
  (set `ProjectileMovementComponent.InitialSpeed` (`self.Initial Speed`) _projectilemovement)
  (set `ProjectileMovementComponent.MaxSpeed` (`self.Initial Speed`) _projectilemovement))

(event `self.Sphere1.OnComponentBeginOverlap`
  (params (OverlappedComponent :type "PrimitiveComponent Object Reference") (OtherActor :type "Actor Object Reference") (OtherComp :type "PrimitiveComponent Object Reference") (OtherBodyIndex :type Integer) (bFromSweep :type Boolean) (SweepResult :type "HitResult Structure (by ref)"))
  (bind _returnvalue (`self.GetComponentByClass` OtherActor "/Game/Marco_Folder/Blueprints/EnemyBlueprints/AC_Health.AC_Health_C"))
  (`/Engine/EditorBlueprintResources/StandardMacros.IsValid` _returnvalue
    (:`Is Valid`
      (`/Game/Marco_Folder/Blueprints/EnemyBlueprints/AC_Health.TakeDamage` _returnvalue (`self.Damage`))
      (`self.K2_DestroyActor`))))

(fn `UserConstructionScript`)