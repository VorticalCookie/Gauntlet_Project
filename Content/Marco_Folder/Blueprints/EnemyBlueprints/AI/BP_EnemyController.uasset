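; Enemy AI controller that runs the enemy behavior tree and decides when the enemy chases or gives up on the player.
; Each tick it checks AI perception of the player pawn and sets the HasSeenPlayer blackboard key while the player is sensed.
; When sight is lost, a one-shot disengage timer starts, guarded by a flag; it clears the key on expiry and is cancelled if the player is sensed again.
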(event `self.ReceiveBeginPlay`
  ;[0 0 0 0.5] Start Running Behavior Tree
  (`self.RunBehaviorTree` "/Game/Marco_Folder/Blueprints/EnemyBlueprints/AI/BT_EnemyBehavior.BT_EnemyBehavior"))

(event `self.ReceiveTick`
  (params (DeltaSeconds :type "Float (single-precision)"))
  ;[0 0 0] Set 'hasBeenSeen' bool on Behavior Tree's Blackboard
  (bind _info (`AIPerceptionComponent.GetActorsPerception` (`self.AIPerception`) (`GameplayStatics.GetPlayerPawn` 0)))
  (if (`.bSuccessfullySensed` (break `AIStimulus` (`|GetArrayItem` (`.LastSensedStimuli` (break `ActorPerceptionBlueprintInfo` _info)))))
    (`BlackboardComponent.SetValueAsBool` (`AIBlueprintHelperLibrary.GetBlackboard` null) "HasSeenPlayer" true)
    (`KismetSystemLibrary.K2_ClearAndInvalidateTimerHandle` (stale _returnvalue))
    (set `self.isDisengaging` false)
    (elif (not (`self.isDisengaging`))
      (bind _returnvalue (`KismetSystemLibrary.K2_SetTimerDelegate` (delegate `Disengage`) (`self.DisengageTime`)))
      (set `self.isDisengaging` true))))

(event `Disengage`
  ;[0 0 0] Stop chasing when player is out of sight for too long
  (`KismetSystemLibrary.PrintString` "Stop Chasing" true true (struct :`G` 0.66 :`B` 1.0 :`A` 1.0) 1.0)
  (`BlackboardComponent.SetValueAsBool` (`AIBlueprintHelperLibrary.GetBlackboard` null) "HasSeenPlayer" false))

(fn `UserConstructionScript`)