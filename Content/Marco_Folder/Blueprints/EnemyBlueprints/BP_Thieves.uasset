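; BP_Thieves is an enemy Blueprint for a thief that makes a melee attack and then flees.
; Its attack interface event calls the parent behavior and spawns a BP_MeleeAttack actor at the AttackPoint, using the thief's rotation.
; It then sets the RunAway blackboard key to true so the AI can switch to escaping.
; Item stealing is only a debug print string here.
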(event `/Game/Marco_Folder/Blueprints/EnemyBlueprints/AI/BPI_Attack.AttackBPI`
  (`parent.AttackBPI`)
  (`|SpawnActorFromClass` "/Game/Marco_Folder/Blueprints/EnemyBlueprints/BP_MeleeAttack.BP_MeleeAttack_C" (`KismetMathLibrary.MakeTransform` (`SceneComponent.K2_GetComponentLocation` (`self.AttackPoint`)) (`self.K2_GetActorRotation`)) "Undefined" "OverrideRootScale" null null)
  (`KismetSystemLibrary.PrintString` "Steal Item")
  (`BlackboardComponent.SetValueAsBool` (`AIBlueprintHelperLibrary.GetBlackboard` null) "RunAway" true))

(fn `UserConstructionScript`
  (`parent.UserConstructionScript`))