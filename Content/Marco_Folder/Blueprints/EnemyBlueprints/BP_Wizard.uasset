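; BP_Wizard is an enemy Blueprint for a wizard that attacks by launching a fireball.
; Its AttackBPI event runs the parent attack, then spawns BP_Fireball at the AttackPoint location, facing the actor's rotation.
; It then hides its Cube and Cone components and shows them again after a short delay.
; The construction script only calls the parent's.
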(event `/Game/Marco_Folder/Blueprints/EnemyBlueprints/AI/BPI_Attack.AttackBPI`
  (`parent.AttackBPI`)
  (`|SpawnActorFromClass` "/Game/Marco_Folder/Blueprints/EnemyBlueprints/BP_Fireball.BP_Fireball_C" (`KismetMathLibrary.MakeTransform` (`SceneComponent.K2_GetComponentLocation` (`self.AttackPoint`)) (`self.K2_GetActorRotation`)) "Undefined" "OverrideRootScale" null null)
  (`SceneComponent.SetVisibility` (`self.Cube`) false false)
  (`SceneComponent.SetVisibility` (`self.Cone`) false false)
  (`KismetSystemLibrary.Delay` 2.0)
  (`SceneComponent.SetVisibility` (`self.Cone`) true false)
  (`SceneComponent.SetVisibility` (`self.Cube`) true false))

(fn `UserConstructionScript`
  (`parent.UserConstructionScript`))