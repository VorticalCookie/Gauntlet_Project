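; BP_EnemyBase is an enemy actor that can drop loot when it dies.
; When its Health component signals death, it runs SpawnLoot and then destroys itself.
; SpawnLoot rolls a percentage against ChanceOfDrop, then spawns a random pick of food, key or potion at the Cube's location, or prints a message when nothing drops.
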(event `Spawn Loot`
  ;[1 1 1] Drop Loot
  (if (<= (`KismetMathLibrary.RandomIntegerInRange` 1 100) (`self.Chance of Drop`))
    (`|SpawnActorFromClass` (select `int` (`KismetMathLibrary.RandomInteger` 3) :`0` "/Game/Marco_Folder/Blueprints/PickupBlueprints/BP_Food.BP_Food_C" :`1` "/Game/Marco_Folder/Blueprints/PickupBlueprints/BP_Key.BP_Key_C" :`2` "/Game/Marco_Folder/Blueprints/PickupBlueprints/BP_Potion.BP_Potion_C" :!type "Actor Class Reference") (`KismetMathLibrary.MakeTransform` (`SceneComponent.K2_GetComponentLocation` (`self.Cube`))) "Undefined" "OverrideRootScale")
    (else
      (`KismetSystemLibrary.PrintString` "No Item Dropped"))))

(event `self.Health_.OnComponentDead`
  (params (causer :type "Controller Object Reference"))
  (`self.Spawn Loot`)
  (`self.K2_DestroyActor`))

(fn `UserConstructionScript`)