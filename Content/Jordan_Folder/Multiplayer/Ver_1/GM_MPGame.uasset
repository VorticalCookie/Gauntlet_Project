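; GM_MPGame is a local multiplayer game mode that sets up extra players and the HUD on BeginPlay.
; A loop creates three local players, each possessing a new BP_ThirdPersonCharacter_P1 spawned at the first existing one's transform; its player-zero branch is never reached.
; It then sets the default pawn class, adds W_HeadsUpDisplay to the viewport and restarts player 0.
; An unconnected alternative setup that indexes and tags BP_Players pawns never runs.
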(event `CustomEvent`)

(event `self.ReceiveBeginPlay`
  (for _index (range 1 4)
    (bind _outactors (`GameplayStatics.GetAllActorsOfClass` "/Game/ThirdPerson/Blueprints/BP_ThirdPersonCharacter_P1.BP_ThirdPersonCharacter_P1_C"))
    (if (> _index 0)
      (bind _returnvalue (`GameplayStatics.CreatePlayer` -1))
      (bind _returnvalue_2 (`self.GetTransform` (`|GetArrayItem` _outactors)))
      (bind _returnvalue_3 (`|SpawnActorFromClass` "/Game/ThirdPerson/Blueprints/BP_ThirdPersonCharacter_P1.BP_ThirdPersonCharacter_P1_C" _returnvalue_2 "Undefined" "OverrideRootScale" null 1 null))
      (`Controller.Possess` _returnvalue _returnvalue_3)
      (else
        (bind _returnvalue_4 (`|SpawnActorFromClass` "/Game/ThirdPerson/Blueprints/BP_ThirdPersonCharacter_P1.BP_ThirdPersonCharacter_P1_C" _returnvalue_2 "Undefined" "OverrideRootScale" null 0 null))
        (`Controller.Possess` (`GameplayStatics.GetPlayerController` 0) _returnvalue_4))))
  (set `self.DefaultPawnClass` "/Game/ThirdPerson/Blueprints/BP_ThirdPersonCharacter_P1.BP_ThirdPersonCharacter_P1_C")
  (bind _returnvalue_5 (`|CreateWidget` "/Game/Jordan_Folder/Game/UI/W_HeadsUpDisplay.W_HeadsUpDisplay_C"))
  (bind _output_get (set `self.HUD` _returnvalue_5))
  (`UserWidget.AddToViewport` _output_get 0)
  (`self.RestartPlayer` (`GameplayStatics.GetPlayerController` 0)))

(fn `UserConstructionScript`)