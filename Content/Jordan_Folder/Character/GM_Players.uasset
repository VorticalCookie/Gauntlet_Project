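; GM_Players is a game mode Blueprint that sets up two local players on BeginPlay.
; It finds existing BP_ThirdPersonCharacter_P1 actors and spawns two new characters at the first one's transform.
; The existing player controller possesses the first spawn.
; A newly created local player controller possesses the second, which receives its own controller index on spawn.
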(event `self.ReceiveBeginPlay`
  (bind _outactors (`GameplayStatics.GetAllActorsOfClass` "/Game/ThirdPerson/Blueprints/BP_ThirdPersonCharacter_P1.BP_ThirdPersonCharacter_P1_C"))
  (for _index (range 2)
    (if (> _index 0)
      (bind _returnvalue (`GameplayStatics.CreatePlayer` -1))
      (bind _returnvalue_2 (`self.GetTransform` (`|GetArrayItem` _outactors)))
      (bind _returnvalue_3 (`|SpawnActorFromClass` "/Game/ThirdPerson/Blueprints/BP_ThirdPersonCharacter_P1.BP_ThirdPersonCharacter_P1_C" _returnvalue_2 "Undefined" "OverrideRootScale" null 1 null))
      (`Controller.Possess` _returnvalue _returnvalue_3)
      (else
        (bind _returnvalue_4 (`|SpawnActorFromClass` "/Game/ThirdPerson/Blueprints/BP_ThirdPersonCharacter_P1.BP_ThirdPersonCharacter_P1_C" _returnvalue_2 "Undefined" "OverrideRootScale" null 0 null))
        (`Controller.Possess` (`GameplayStatics.GetPlayerController` 0) _returnvalue_4)))))

(fn `UserConstructionScript`)